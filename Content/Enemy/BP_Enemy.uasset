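; BP_Enemy is an enemy actor that travels along a level spline and dies when a projectile hits it.
; On BeginPlay it finds BP_Spline and plays a timeline, with play rate set by TimeAction, to set world location and local-space rotation from distance along the spline.
; When its Box overlaps a BP_Projectile, it calls EnemyDead on BP_GameInstance and destroys itself.
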(event `self.ReceiveBeginPlay`
  (bind _returnvalue (`GameplayStatics.GetActorOfClass` "/Game/Enemy/BP_Spline.BP_Spline_C"))
  (set `self.SplineREF` _returnvalue)
  (`self.Move Object`))

(event `Move Object`
  (bind _spline (`/Game/Enemy/BP_Spline.Spline` (`self.SplineREF`)))
  (`TimelineComponent.SetPlayRate` (`self.Move Object T`) (/ 1.0 (`self.TimeAction`)))
  (bind (_direction _movetrack) (`Timeline|Move Object T`)
    (:`Update`
      (bind _returnvalue (`KismetMathLibrary.Lerp` 0.0 (`SplineComponent.GetSplineLength` (`/Game/Enemy/BP_Spline.Spline` (`self.SplineREF`))) _movetrack))
      (`self.K2_SetActorTransform` (`KismetMathLibrary.MakeTransform` (`SplineComponent.GetLocationAtDistanceAlongSpline` _spline _returnvalue "World") (`SplineComponent.GetRotationAtDistanceAlongSpline` _spline _returnvalue "Local"))))))

(event `self.Box.OnComponentBeginOverlap`
  (params (OverlappedComponent :type "PrimitiveComponent Object Reference") (OtherActor :type "Actor Object Reference") (OtherComp :type "PrimitiveComponent Object Reference") (OtherBodyIndex :type Integer) (bFromSweep :type Boolean) (SweepResult :type "HitResult Structure (by ref)"))
  (cast `/Game/Projectile/BP_Projectile` OtherActor)
  (`/Game/GameManager/BP_GameInstance.EnemyDead` (cast `/Game/GameManager/BP_GameInstance` (`GameplayStatics.GetGameInstance`) :!pure true))
  (`self.K2_DestroyActor`))

(fn `UserConstructionScript`)