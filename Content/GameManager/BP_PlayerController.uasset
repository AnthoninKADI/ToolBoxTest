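; Player controller that turns Enhanced Input actions into movement, camera look, sprint and crouch for the controlled pawn.
; BeginPlay adds the default mapping context and limits camera pitch; move input follows the control rotation, and look input inverts Y for pitch.
; Sprint swaps max walk speed between the pawn's run and walk values, while crouch is held.
; The pawn casts that sprint and crouch read from are never executed.
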(event Input|EnhancedActionEvents|EnhancedInputActionIA_Move
  (params (ActionValue :type Vector%202D%20Structure) (ElapsedSeconds :type Float%20%28double-precision%29) (TriggeredSeconds :type Float%20%28double-precision%29) (InputAction :type Input%20Action%20Object%20Reference :default "/Game/Input/IA/IA_Move.IA_Move"))
  (bind _returnvalue (Pawn|GetControlRotation :!class /Script/Engine.Controller))
  (bind _returnvalue_2 (Pawn|GetControlledPawn))
  ;[0 0.6331 1] Movement
  (Pawn|Input|AddMovementInput _returnvalue_2 (Math|Vector|GetForwardVector _returnvalue) (.x ActionValue) false)
  (Pawn|Input|AddMovementInput _returnvalue_2 (Math|Vector|GetRightVector _returnvalue) (.y ActionValue) false))

(event Input|EnhancedActionEvents|EnhancedInputActionIA_Camera
  (params (ActionValue :type Vector%202D%20Structure) (ElapsedSeconds :type Float%20%28double-precision%29) (TriggeredSeconds :type Float%20%28double-precision%29) (InputAction :type Input%20Action%20Object%20Reference :default "/Game/Input/IA/IA_Camera.IA_Camera"))
  ;[0 0.6331 1] Movement
  (Class|PlayerController|AddYawInput (.x ActionValue))
  (Class|PlayerController|AddPitchInput (* (.y ActionValue) -1.0)))

(event Input|EnhancedActionEvents|EnhancedInputActionIA_Sprint
  (params (ActionValue :type Boolean) (ElapsedSeconds :type Float%20%28double-precision%29) (TriggeredSeconds :type Float%20%28double-precision%29) (InputAction :type Input%20Action%20Object%20Reference :default "/Game/Input/IA/IA_Sprint.IA_Sprint"))
  ;[1 0 0.6819] Sprint
  (:Triggered
    (Variables|/Script/Engine.CharacterMovementComponent|SetMaxWalkSpeed (Variables|/Script/Engine.Character|GetCharacterMovement (stale _asbp_player)) (Variables|Default|GetRunSpeed (stale _asbp_soldier))))
  (:Completed
    (Variables|/Script/Engine.CharacterMovementComponent|SetMaxWalkSpeed (Variables|/Script/Engine.Character|GetCharacterMovement (stale _asbp_player)) (Variables|Default|GetWalkSpeed (stale _asbp_soldier)))))

(event Input|EnhancedActionEvents|EnhancedInputActionIA_Crouch
  (params (ActionValue :type Boolean) (ElapsedSeconds :type Float%20%28double-precision%29) (TriggeredSeconds :type Float%20%28double-precision%29) (InputAction :type Input%20Action%20Object%20Reference :default "/Game/Input/IA/IA_Crouch.IA_Crouch"))
  ;[1 0.7676 0] Crouch
  (:Triggered
    (Character|Crouch (stale _asbp_soldier)))
  (:Completed
    (Character|UnCrouch (stale _asbp_soldier))))

(event EventBeginPlay
  (bind _returnvalue (Game|GetPlayerCameraManager 0))
  ;[0 0.6331 1] Movement
  (Input|AddMappingContext (PlayerController|LocalPlayerSubsystems|GetEnhancedInputLocalPlayerSubsystem) "/Game/Input/IMC_Default.IMC_Default" 0 "(bIgnoreAllPressedKeysUntilRelease=True,bForceImmediately=False,bNotifyUserSettings=False)")
  (Variables|/Script/Engine.PlayerCameraManager|SetViewPitchMax _returnvalue 6e+01)
  (Variables|/Script/Engine.PlayerCameraManager|SetViewPitchMin _returnvalue -2e+01))

(fn ConstructionScript)